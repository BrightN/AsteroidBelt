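; BP_StarField is an actor that generates a random star field at BeginPlay and makes itself the player's view target in unlit viewmode.
; Init creates a BP_DrawingCanvas and feeds its dynamic texture into a material instance on the Canvas component.
; It sizes that component and the camera's ortho width from the pixel dimensions.
; DrawDecals then stamps three star textures at random pixel coordinates on the texture.
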(event `self.ReceiveBeginPlay`
  (`KismetSystemLibrary.ExecuteConsoleCommand` "viewmode unlit" null)
  (`PlayerController.SetViewTargetWithBlend` (`GameplayStatics.GetPlayerController` 0) self 0.0 "VTBlend_Linear" 0.0 false) ; Setup Camera
  (`self.Init`))

(fn `DrawDecals`
  (params (DecalTexture :type "Texture2D Object Reference") (DecalsNum :type Integer :default 300))
  (locals (NewLocalVar_0 :type "Texture2D Object Reference" :default "Texture2D'/Game/Sprites/star0.star0'"))
  (`DrawingCanvas.InitializeDecal` (`self.DrawingCanvas`) DecalTexture)
  (for _ (range 1 (+ DecalsNum 1))
    (`DrawingCanvas.DrawDecal` (`self.DrawingCanvas`) (`KismetMathLibrary.RandomInteger` (`self.Width`)) (`KismetMathLibrary.RandomInteger` (`self.Height`)))))

(fn `Init`
  (`|ExecutionSequence`
    (:`then_0`
      ;[1 1 1] Init Drawing Canvas
      (bind _returnvalue (`|GenericCreateObject` "/Game/Blueprints/BP_DrawingCanvas.BP_DrawingCanvas_C" self))
      (bind _output_get (set `self.DrawingCanvas` _returnvalue))
      (`DrawingCanvas.InitializeCanvas` _output_get (`self.Width`) (`self.Height`)))
    (:`then_1`
      ;[1 1 1] Init Drawing Canvas Material
      (bind _returnvalue_2 (`PrimitiveComponent.CreateDynamicMaterialInstance` (`self.Canvas`) 0 null "None"))
      (bind _output_get_2 (set `self.CanvasMID` _returnvalue_2))
      (`MaterialInstanceDynamic.SetTextureParameterValue` _output_get_2 "TextureInput" (`DrawingCanvas.dynamicCanvas` (`self.DrawingCanvas`))))
    (:`then_2`
      ;[1 1 1] Init Objects
      (`SceneComponent.SetRelativeScale3D` (`self.Canvas`) (`KismetMathLibrary.MakeVector` (`KismetMathLibrary.Conv_IntToDouble` (/ (`self.Width`) 100)) (`KismetMathLibrary.Conv_IntToDouble` (/ (`self.Height`) 100))))
      (`CameraComponent.SetOrthoWidth` (`self.Camera`) (`KismetMathLibrary.Conv_IntToDouble` (`self.Width`))))
    (:`then_3`
      (`self.DrawDecals` "/Game/Sprites/star0.star0")
      (`self.DrawDecals` "/Game/Sprites/star1.star1")
      (`self.DrawDecals` "/Game/Sprites/star2.star2"))))

(fn `UserConstructionScript`)